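; MainCrystalBlueprint is a crystal drop-off point that banks the crystals the player is carrying.
; Every Tick, it checks whether CrystalPlaceTrigger overlaps the player character and casts that character to MyPlayerPrototype.
; It then adds the player's Crystals to CrystalsReturned and resets Crystals to zero, behind a branch that is always true.
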(event EventBeginPlay)

(event Collision|EventActorBeginOverlap
  (params (OtherActor :type Actor%20Object%20Reference)))

(event EventTick
  (params (DeltaSeconds :type Float%20%28single-precision%29))
  (bind _returnvalue (Game|GetPlayerCharacter 0))
  (if (Collision|IsOverlappingActor (Variables|Default|GetCrystal%20Place%20Trigger) _returnvalue :!class /Script/Engine.PrimitiveComponent)
    (bind _asmy_player_prototype (Utilities|Casting|CastToMyPlayerPrototype _returnvalue))
    (if true
      (Variables|/Game/SeanPrototypes/Blueprints/MyPlayerPrototype.MyPlayerPrototype_C|SetCrystalsReturned _asmy_player_prototype (+ (Variables|/Game/SeanPrototypes/Blueprints/MyPlayerPrototype.MyPlayerPrototype_C|GetCrystals _asmy_player_prototype) (Variables|/Game/SeanPrototypes/Blueprints/MyPlayerPrototype.MyPlayerPrototype_C|GetCrystalsReturned _asmy_player_prototype)))
      (Variables|/Game/SeanPrototypes/Blueprints/MyPlayerPrototype.MyPlayerPrototype_C|SetCrystals _asmy_player_prototype 0))))

(fn ConstructionScript)