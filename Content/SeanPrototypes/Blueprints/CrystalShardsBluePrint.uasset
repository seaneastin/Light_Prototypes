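; Crystal shard pickup that adds one to the player's crystal count when collected.
; Each Tick polls PickupCollision for overlap with player pawn 0 instead of using overlap events.
; On overlap it casts to MyPlayerPrototype, increments Crystals and prints the new total.
; An IsCollected flag blocks repeat pickups, and the actor moves to the world origin rather than being destroyed.
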(event EventBeginPlay)

(event Collision|EventActorBeginOverlap
  (params (OtherActor :type Actor%20Object%20Reference)))

(event EventTick
  (params (DeltaSeconds :type Float%20%28single-precision%29))
  (bind _returnvalue (Game|Player|GetPlayerPawn 0))
  (if (not (Variables|Default|GetIs%20Collected))
    (if (Collision|IsOverlappingActor (Variables|Default|Getpickup%20collision) _returnvalue :!class /Script/Engine.PrimitiveComponent)
      (bind _asmy_player_prototype (Utilities|Casting|CastToMyPlayerPrototype _returnvalue))
      (Development|PrintString (Utilities|String|BuildString(Integer) "" "player now has" (+ (Variables|/Game/SeanPrototypes/Blueprints/MyPlayerPrototype.MyPlayerPrototype_C|GetCrystals _asmy_player_prototype) 1) "crystals"))
      (Variables|/Game/SeanPrototypes/Blueprints/MyPlayerPrototype.MyPlayerPrototype_C|SetCrystals _asmy_player_prototype (+ (Variables|/Game/SeanPrototypes/Blueprints/MyPlayerPrototype.MyPlayerPrototype_C|GetCrystals _asmy_player_prototype) 1))
      (Variables|Default|SetIs%20Collected true)
      (Transformation|SetActorLocation "0, 0, 0" false false))))

(fn ConstructionScript)